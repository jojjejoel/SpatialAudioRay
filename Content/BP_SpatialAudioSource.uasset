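; BP_SpatialAudioSource is an actor Blueprint that, by its name, serves as a spatial audio source, though its graphs contain no audio logic.
; BeginPlay stores a DestinationLocation offset along X from the root component's relative location, and nothing shown reads it.
; An unconnected chain would move the actor along X and reverse XVelocity beyond a distance from the world origin.
; Tick is empty, so the graphs never move the actor.
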(event `self.ReceiveBeginPlay`
  (set `self.DestinationLocation` (+ (`SceneComponent.RelativeLocation` (`self.RootComponent`)) (100.0 0.0 0.0))))

(event `self.ReceiveTick`
  (params (DeltaSeconds :type "Float (single-precision)")))

(fn `UserConstructionScript`)